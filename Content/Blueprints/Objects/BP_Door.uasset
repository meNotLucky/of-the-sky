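; Interactable bridge door that swings BridgePivot 90 degrees open or closed, on roll or yaw depending on its direction setting.
; OnInteraction sets the target rotation and a pending flag, which Tick consumes by interpolating the pivot until it is nearly there.
; The first opening blends the view to the bridge and disables player input; finishing an opening restores both.
; Construction syncs the activation sound delay to the drop delay.
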(event `self.ReceiveTick`
  (params (DeltaSeconds :type "Float (single-precision)"))
  (if (`self.isOpen`)
    (if (`self.closeBridge`)
      (`self.SetBridge`
        (:`End`
          (set `self.isOpen` false)
          (set `self.closeBridge` false))))
    (elif (`self.openBridge`)
      (if (not (`self.cameraPanned`))
        (`/Engine/EditorBlueprintResources/StandardMacros.DoOnce` false
          (:`Completed`
            (`self.CameraPanToBridge`)
            (`KismetSystemLibrary.Delay` (`self.delayUntilDrop`))
            (set `self.cameraPanned` true))))
      (`self.SetBridge`
        (:`End`
          (`self.CameraPanToCharacter`)
          (set `self.isOpen` true)
          (set `self.openBridge` false))))))

(fn `CameraPanToBridge`
  (`PlayerController.SetViewTargetWithBlend` (`GameplayStatics.GetPlayerController` 0) self (`self.blendToBridge`) "VTBlend_Linear" 0.0 false)
  (`self.DisableInput` (`GameplayStatics.GetPlayerCharacter` 0) (`GameplayStatics.GetPlayerController` 0)))

(fn `CameraPanToCharacter`
  (`PlayerController.SetViewTargetWithBlend` (`GameplayStatics.GetPlayerController` 0) (`GameplayStatics.GetPlayerPawn` 0) (`self.blendToPlayer`) "VTBlend_Linear" 0.0 false)
  (`self.EnableInput` (`GameplayStatics.GetPlayerCharacter` 0) (`GameplayStatics.GetPlayerController` 0)))

(fn `OnInteraction`
  (bind _returnvalue (== (`self.opencloseDirection`) (enumliteral `/Game/Blueprints/Objects/Utility/E_Direction` "NewEnumerator1")))
  (bind (_returnvalue_roll _returnvalue_pitch _returnvalue_yaw) (`KismetMathLibrary.BreakRotator` (`SceneComponent.K2_GetComponentRotation` (`self.BridgePivot`))))
  (bind (_open _close) (`self.GetRotation` (`self.BridgePivot`)))
  (if (`self.isOpen`)
    (if (not (`self.closeBridge`))
      (set `self.closeBridge` true)
      (if _returnvalue
        (set `self.targetRotation` _open)
        (else
          (set `self.targetRotation` (`KismetMathLibrary.MakeRotator` _returnvalue_roll _returnvalue_pitch (+ _returnvalue_yaw 90.0))))))
    (elif (not (`self.openBridge`))
      (set `self.openBridge` true)
      (if _returnvalue
        (set `self.targetRotation` _close)
        (else
          (set `self.targetRotation` (`KismetMathLibrary.MakeRotator` _returnvalue_roll _returnvalue_pitch (- _returnvalue_yaw 90.0))))))))

(fn `UserConstructionScript`
  (`parent.UserConstructionScript`)
  (set `self.activationSoundDelay` (`self.delayUntilDrop`)))