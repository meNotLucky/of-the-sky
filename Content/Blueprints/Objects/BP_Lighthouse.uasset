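; BP_Lighthouse is an interactable lighthouse object whose arm pitches to a new angle when the player interacts with it.
; OnInteraction extends the parent logic, turns off the outline, locks the object and sets a target rotation pitched up from the Arm's current world rotation.
; While IsActive is true, Tick turns the Arm's relative rotation toward that target at constant speed.
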(event `self.ReceiveTick`
  (params (DeltaSeconds :type "Float (single-precision)"))
  (if (`self.isActive`)
    (`SceneComponent.K2_SetRelativeRotation` (`self.Arm`) (`KismetMathLibrary.RInterpTo_Constant` (`SceneComponent.RelativeRotation` (`self.Arm`)) (`self.targetRotation`) (`GameplayStatics.GetWorldDeltaSeconds`) 5.0) false false)))

(fn `OnInteraction`
  (bind (_returnvalue_roll _returnvalue_pitch _returnvalue_yaw) (`KismetMathLibrary.BreakRotator` (`SceneComponent.K2_GetComponentRotation` (`self.Arm`))))
  (`parent.OnInteraction`)
  (`self.RenderOutline` false)
  (`self.SetLocked` true)
  (set `self.targetRotation` (`KismetMathLibrary.MakeRotator` _returnvalue_roll (+ _returnvalue_pitch 40.0) _returnvalue_yaw)))

(fn `UserConstructionScript`
  (`parent.UserConstructionScript`))