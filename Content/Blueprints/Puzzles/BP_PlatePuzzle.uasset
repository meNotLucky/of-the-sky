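; Pressure plate puzzle actor that is solved by matching plate states to a sequence of combinations.
; Until solved, Tick compares each child actor's active state against the current combination's map, keyed by component name.
; A match activates that combination's trigger objects, locks and dims the plates, and plays a win sound.
; After a delay it resets the plates and advances to the next combination, staying completed after the last.
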(event `self.ReceiveTick`
  (params (DeltaSeconds :type "Float (single-precision)"))
  (bind _output_combination (break `/Game/Blueprints/Puzzles/S_PuzzleCombination` (`|GetArrayItem` (`self.combinations`) (`self.combinationIndex`))))
  ;[1 1 1] Check Combination
  (if (not (`self.isCompleted`))
    (set `self.isCompleted` true)
    (for _array_element (`self.K2_GetComponentsByClass` "/Script/Engine.ChildActorComponent")
      (bind _asbp_interactable_object (cast `/Game/Blueprints/Objects/Utility/BP_InteractableObject` (`ChildActorComponent.ChildActor` _array_element)))
      (if (`/Game/Blueprints/Objects/Utility/BP_InteractableObject.isActive` _asbp_interactable_object)
        (bind (_value _returnvalue) (`BlueprintMapLibrary.Map_Find` _output_combination (`KismetSystemLibrary.GetObjectName` _array_element)))
        (if _returnvalue
          (if (not _value)
            (set `self.isCompleted` false))
          (else
            (`KismetSystemLibrary.PrintString` (`KismetStringLibrary.Concat_StrStr` "One or more order values are incorrect in: " (`KismetSystemLibrary.GetObjectName` self)) true true (struct :`R` 0.473958 :`B` 0.002865 :`A` 1.0) 0.1)))
        (elif _value
          (set `self.isCompleted` false))))
    (`self.Check Complete Condition`)))

(event `Check Complete Condition`
  ;[1 1 1] Check Combination
  (if (`self.isCompleted`)
    (`self.Completed`)))

(event `Reset Puzzle`
  ;[1 1 1] Reset
  (for _array_element (`self.K2_GetComponentsByClass` "/Script/Engine.ChildActorComponent")
    (bind _asbp_pressure_plate (cast `/Game/Blueprints/Objects/BP_PressurePlate` (`ChildActorComponent.ChildActor` _array_element)))
    (set `/Game/Blueprints/Objects/Utility/BP_InteractableObject.isActive` false _asbp_pressure_plate)
    (`/Game/Blueprints/Objects/Utility/BP_InteractableObject.SetLocked` _asbp_pressure_plate false)
    (`/Game/Blueprints/Objects/Utility/BP_InteractableObject.RenderOutline` _asbp_pressure_plate false false)))

(event `Completed`
  (bind (_output_combination _output_triggerobjects) (break `/Game/Blueprints/Puzzles/S_PuzzleCombination` (`|GetArrayItem` (`self.combinations`) (`self.combinationIndex`))))
  ;[1 1 1] Completed
  (for _array_element _output_triggerobjects
    (`/Game/Blueprints/Objects/Utility/BP_InteractableObject.Activate` _array_element)
    (for _array_element_2 (`self.K2_GetComponentsByClass` "/Script/Engine.ChildActorComponent")
      (bind _asbp_pressure_plate (cast `/Game/Blueprints/Objects/BP_PressurePlate` (`ChildActorComponent.ChildActor` _array_element_2)))
      (`/Game/Blueprints/Objects/Utility/BP_InteractableObject.SetLocked` _asbp_pressure_plate true)
      (`MaterialInstanceDynamic.SetScalarParameterValue` (`/Game/Blueprints/Objects/BP_PressurePlate.dynamicMaterial` _asbp_pressure_plate) "GlowStrenght" 0.0)))
  (`GameplayStatics.PlaySound2D` (`self.Puzzle Win Sound`) 1.0 1.0 0.0 null null)
  (`KismetSystemLibrary.Delay` (`self.delayToReset`))
  (`self.Reset Puzzle`)
  (if (< (`self.combinationIndex`) (- (`KismetArrayLibrary.Array_Length` (`self.combinations`)) 1))
    (`/Engine/EditorBlueprintResources/StandardMacros.IncrementInt` (`self.combinationIndex`)
      (:`  `
        (set `self.isCompleted` false)))))

(fn `UserConstructionScript`)