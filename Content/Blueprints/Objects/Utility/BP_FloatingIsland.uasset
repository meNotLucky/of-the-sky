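; Interactable floating island that moves to an end position in a short cutscene, triggered by interaction or, optionally, by completed runes in BP_GameState.
; Tick polls the trigger, then blends the view to the island and disables player input.
; A timeline lerps a Scene child component toward EndPositon, with optional world camera shake.
; On arrival the view blends back to the player and input returns after the blend.
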(event `Enable Player Controls`
  (`KismetSystemLibrary.Delay` (`self.blendToPlayer`))
  (`self.EnableInput` (`GameplayStatics.GetPlayerCharacter` 0) (`GameplayStatics.GetPlayerController` 0)))

(event `self.ReceiveTick`
  (params (DeltaSeconds :type "Float (single-precision)"))
  (`self.CheckRunes`)
  (if (`self.moveUp`)
    (if (not (`self.cameraPanned`))
      (`/Engine/EditorBlueprintResources/StandardMacros.DoOnce` false
        (:`Completed`
          (`self.CameraPanToIsland`)
          (`KismetSystemLibrary.Delay` (`self.delayToSeeIslandMove`))
          (set `self.cameraPanned` true))))
    (for _array_element (`SceneComponent.GetChildrenComponents` (`self.Scene`) false)
      (if (!= _array_element (`self.EndPositon`))
        (`/Engine/EditorBlueprintResources/StandardMacros.DoOnce` false
          (:`Completed`
            (set `self.originalPosition` (`SceneComponent.K2_GetComponentLocation` _array_element))
            (bind (_direction _alpha) (`Timeline|Interpolation`)
              (:`Update`
                (`SceneComponent.K2_SetWorldLocation` _array_element (`KismetMathLibrary.VLerp` (`self.originalPosition`) (`SceneComponent.K2_GetComponentLocation` (`self.EndPositon`)) _alpha) false false))
              (:`Finished`
                (set `self.destinationReached` true)))))))
    (if (`self.cameraShake`)
      (`self.Activate Shake`))
    (if (`self.destinationReached`)
      (`/Engine/EditorBlueprintResources/StandardMacros.DoOnce` false
        (:`Completed`
          (`self.CameraPanToCharacter`))))))

(event `CheckRunes`
  (bind _asbp_game_state (cast `/Game/Blueprints/BP_GameState` (`GameplayStatics.GetGameState`)))
  (if (and (`self.completedOnRunesCollected`) (`/Game/Blueprints/BP_GameState.runesCompleted` _asbp_game_state))
    (set `self.moveUp` true)
    (set `self.isLocked` true)))

(event `Activate Shake`
  (`/Engine/EditorBlueprintResources/StandardMacros.DoOnce` false
    (:`Completed`
      (`GameplayStatics.PlayWorldCameraShake` (`self.shake`) (`SceneComponent.K2_GetComponentLocation` (`self.Camera`)) 0.0 10000.0))))

(fn `CameraPanToCharacter`
  (`PlayerController.SetViewTargetWithBlend` (`GameplayStatics.GetPlayerController` 0) (`GameplayStatics.GetPlayerPawn` 0) (`self.blendToPlayer`) "VTBlend_EaseInOut" 3.0 false)
  (`self.Enable Player Controls`))

(fn `CameraPanToIsland`
  (`PlayerController.SetViewTargetWithBlend` (`GameplayStatics.GetPlayerController` 0) self (`self.blendToIsland`) "VTBlend_EaseInOut" 3.0 false)
  (`self.DisableInput` (`GameplayStatics.GetPlayerCharacter` 0) (`GameplayStatics.GetPlayerController` 0)))

(fn `OnInteraction`
  (set `self.moveUp` true)
  (set `self.isLocked` true))

(fn `UserConstructionScript`
  (`parent.UserConstructionScript`)
  (set `self.activationSoundDelay` (`self.delayToSeeIslandMove`)))