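; BP_Drawbridge is an interactable drawbridge that swings open or closed by rolling its pivot component 90 degrees.
; OnInteraction sets a target rotation and a pending open or close flag, ignoring repeat calls in the same direction until the move finishes.
; While a flag is set, Tick runs SetBridge, which eases the pivot with RInterpTo.
; Within one degree of the target, Tick flips IsOpen and clears the flag.
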(event `self.ReceiveTick`
  (params (DeltaSeconds :type "Float (single-precision)"))
  (if (`self.isOpen`)
    (if (`self.closeBridge`)
      (`self.SetBridge`
        (:`End`
          (set `self.isOpen` false)
          (set `self.closeBridge` false))))
    (elif (`self.openBridge`)
      (`self.SetBridge`
        (:`End`
          (set `self.isOpen` true)
          (set `self.openBridge` false))))))

(fn `OnInteraction`
  (bind (_returnvalue_roll _returnvalue_pitch _returnvalue_yaw) (`KismetMathLibrary.BreakRotator` (`SceneComponent.K2_GetComponentRotation` (`self.BridgePivot`))))
  (if (`self.isOpen`)
    (if (not (`self.closeBridge`))
      (set `self.closeBridge` true)
      (set `self.targetRotation` (`KismetMathLibrary.MakeRotator` (+ _returnvalue_roll 90.0) _returnvalue_pitch _returnvalue_yaw)))
    (elif (not (`self.openBridge`))
      (set `self.openBridge` true)
      (set `self.targetRotation` (`KismetMathLibrary.MakeRotator` (- _returnvalue_roll 90.0) _returnvalue_pitch _returnvalue_yaw)))))

(fn `UserConstructionScript`
  (`parent.UserConstructionScript`))