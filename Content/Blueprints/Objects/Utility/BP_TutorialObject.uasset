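; BP_TutorialObject is an interactable trigger that shows a tutorial prompt for walking, sprinting, jumping, gliding or camera control.
; Tick polls player overlap with the collider and calls Activate once the game has started and no widget is valid.
; On interaction, it creates WB_Tutorial, reveals the section matching its Tutorial value and locks itself.
; The prompt is removed on overlap end, or after a one-time delay when EndAfterTime is set.
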(event `OverlapCheck`
  (if (`PrimitiveComponent.IsOverlappingActor` (`self.Collider`) (`GameplayStatics.GetPlayerCharacter` 0))
    (bind _asbp_game_state (cast `/Game/Blueprints/BP_GameState` (`GameplayStatics.GetGameState`)))
    (if (`/Game/Blueprints/BP_GameState.gameStarted` _asbp_game_state)
      (`/Engine/EditorBlueprintResources/StandardMacros.IsValid` (`self.widget`)
        (:`Is Not Valid`
          (`self.Activate`))))))

(event `self.Collider.OnComponentEndOverlap`
  (params (OverlappedComponent :type "PrimitiveComponent Object Reference") (OtherActor :type "Actor Object Reference") (OtherComp :type "PrimitiveComponent Object Reference") (OtherBodyIndex :type Integer))
  (bind _widget (`self.widget`))
  (if (== OtherActor (`GameplayStatics.GetPlayerCharacter` 0))
    (if (not (`self.endAfterTime`))
      (`/Engine/EditorBlueprintResources/StandardMacros.IsValid` _widget
        (:`Is Valid`
          (`Widget.RemoveFromParent` _widget))))))

(event `self.ReceiveTick`
  (params (DeltaSeconds :type "Float (single-precision)"))
  (bind _widget (`self.widget`))
  (`self.OverlapCheck`)
  (if (`self.isActive`)
    (`/Engine/EditorBlueprintResources/StandardMacros.DoOnce` false
      (:`Completed`
        (if (`self.endAfterTime`)
          (`KismetSystemLibrary.Delay` (`self.timeToEnd`))
          (`/Engine/EditorBlueprintResources/StandardMacros.IsValid` _widget
            (:`Is Valid`
              (`Widget.RemoveFromParent` _widget))))))))

(fn `OnInteraction`
  (`parent.OnInteraction`)
  (bind _returnvalue (`|CreateWidget` "/Game/Blueprints/UI/WB_Tutorial.WB_Tutorial_C"))
  (bind _output_get (set `self.widget` _returnvalue))
  (`UserWidget.AddToViewport` _output_get 0)
  (`self.SetLocked` true)
  (switch `/Game/Blueprints/Objects/Utility/E_TutorialTypes` (`self.tutorial`)
    (:`NewEnumerator0`
      (set `/Game/Blueprints/UI/WB_Tutorial.walkVisibility` "Visible" _returnvalue))
    (:`NewEnumerator1`
      (set `/Game/Blueprints/UI/WB_Tutorial.sprintVisibility` "Visible" _returnvalue))
    (:`NewEnumerator2`
      (set `/Game/Blueprints/UI/WB_Tutorial.jumpVisibility` "Visible" _returnvalue))
    (:`NewEnumerator3`
      (set `/Game/Blueprints/UI/WB_Tutorial.glideVisibility` "Visible" _returnvalue))
    (:`NewEnumerator4`
      (set `/Game/Blueprints/UI/WB_Tutorial.cameraVisibility` "Visible" _returnvalue))))

(fn `UserConstructionScript`
  (`parent.UserConstructionScript`))