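; BP_CamerraBox is a trigger box that plays a short camera cutaway when the player's pawn enters it.
; On overlap it blends the view target to itself and disables the player character's input.
; After a configurable hold time it blends back to the pawn and restores input once the return blend finishes.
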(event `self.Box.OnComponentBeginOverlap`
  (params (OverlappedComponent :type "PrimitiveComponent Object Reference") (OtherActor :type "Actor Object Reference") (OtherComp :type "PrimitiveComponent Object Reference") (OtherBodyIndex :type Integer) (bFromSweep :type Boolean) (SweepResult :type "HitResult Structure (by ref)"))
  ;[1 1 1] Camera Transition 1
  (if (== OtherActor (`GameplayStatics.GetPlayerPawn` 0))
    (`PlayerController.SetViewTargetWithBlend` (`GameplayStatics.GetPlayerController` 0) self (`self.blendTimeIn`) "VTBlend_Linear" 0.0 false)
    (`self.DisableInput` (`GameplayStatics.GetPlayerCharacter` 0) (`GameplayStatics.GetPlayerController` 0))
    (`KismetSystemLibrary.Delay` (`self.cameraStoppedTime`))
    (`PlayerController.SetViewTargetWithBlend` (`GameplayStatics.GetPlayerController` 0) (`GameplayStatics.GetPlayerPawn` 0) (`self.blendTimeOut`) "VTBlend_Linear" 0.0 false)
    (`KismetSystemLibrary.Delay` (`self.blendTimeOut`))
    (`self.EnableInput` (`GameplayStatics.GetPlayerCharacter` 0) (`GameplayStatics.GetPlayerController` 0))))

(fn `UserConstructionScript`)