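; Player spawn manager that returns player 0 to a recently recorded position after a fall.
; Each Tick traces 1000 units down from the player, with the debug line drawn.
; A hit closer than 100 units saves the player's location after a short Delay, read when the Delay ends.
; No hit leads, after a one-second Delay, to Death, which moves the player to LastPosition without rechecking for ground.
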(event `self.ReceiveTick`
  (params (DeltaSeconds :type "Float (single-precision)"))
  (bind _rootcomponent (`Actor.RootComponent` (`GameplayStatics.GetPlayerCharacter` 0)))
  (bind _returnvalue (`SceneComponent.K2_GetComponentLocation` _rootcomponent))
  (bind _outhit (`KismetSystemLibrary.LineTraceSingle` :`Start` _returnvalue :`End` (+ (* (`SceneComponent.GetUpVector` _rootcomponent) -1000.0) _returnvalue) :`TraceChannel` "TraceTypeQuery1" :`DrawDebugType` "ForOneFrame"))
  (if (`GameplayStatics.BreakHitResult` _outhit)
    (if (< (`.Distance` (`GameplayStatics.BreakHitResult` _outhit)) 100.0)
      (`KismetSystemLibrary.Delay` 0.2)
      (set `self.Last Position` (`SceneComponent.K2_GetComponentLocation` (`Actor.RootComponent` (`GameplayStatics.GetPlayerCharacter` 0)))))
    (else
      (`KismetSystemLibrary.Delay` 1.0)
      (`self.Death`))))

(event `Death`
  (`SceneComponent.K2_SetWorldLocation` (`Actor.RootComponent` (`GameplayStatics.GetPlayerCharacter` 0)) (`self.Last Position`) false false))

(fn `UserConstructionScript`)