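; Base interactable object that responds to the player entering or leaving its collider, with empty OnInteraction and AfterInteraction hooks.
; Overlaps either activate and deactivate it directly or add and remove it from the player's InteractableObjectsInRange, per ActivationOnCollision.
; Toggle objects flip on each entry based on IsActive; others reverse on exit.
; Unless locked, activation plays an optional sound and drives a custom-depth outline and GameState's HUD prompt.
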(event `self.Collider.OnComponentBeginOverlap`
  (params (OverlappedComponent :type "PrimitiveComponent Object Reference") (OtherActor :type "Actor Object Reference") (OtherComp :type "PrimitiveComponent Object Reference") (OtherBodyIndex :type Integer) (bFromSweep :type Boolean) (SweepResult :type "HitResult Structure (by ref)"))
  (bind _returnvalue (`GameplayStatics.GetPlayerCharacter` 0))
  (if (== OtherActor _returnvalue)
    (if (`self.isToggle`)
      (if (`self.isActive`)
        (if (`self.activationOnCollision`) :!label _label
          (`self.Deactivate`)
          (else
            (bind _asbp_player_character (cast `/Game/Blueprints/Character/BP_PlayerCharacter` _returnvalue)
              (:`then`
                (`KismetArrayLibrary.Array_RemoveItem` (`/Game/Blueprints/Character/BP_PlayerCharacter.interactableObjectsInRange` _asbp_player_character) self))
              (:`CastFailed`
                (`KismetSystemLibrary.PrintString` "Player Character Cast Failed!")))))
        (else
          (if (`self.activationOnCollision`) :!label _label_2
            (`self.Activate`)
            (else
              (bind _asbp_player_character_2 (cast `/Game/Blueprints/Character/BP_PlayerCharacter` _returnvalue)
                (:`then`
                  (`KismetArrayLibrary.Array_Add` (`/Game/Blueprints/Character/BP_PlayerCharacter.interactableObjectsInRange` _asbp_player_character_2) self))
                (:`CastFailed`
                  (`KismetSystemLibrary.PrintString` "Player Character Cast Failed!")))))))
      (else
        (goto _label_2)))))

(event `self.Collider.OnComponentEndOverlap`
  (params (OverlappedComponent :type "PrimitiveComponent Object Reference") (OtherActor :type "Actor Object Reference") (OtherComp :type "PrimitiveComponent Object Reference") (OtherBodyIndex :type Integer))
  (if (== OtherActor (`GameplayStatics.GetPlayerCharacter` 0))
    (if (not (`self.isToggle`))
      (goto _label))))

(fn `Activate`
  (if (not (`self.isLocked`))
    (`self.RenderOutline` true)
    (`self.OnInteraction`)
    (if (not (`self.isActive`))
      (set `self.isActive` true)
      (if (not (== (`self.soundOnActivation`) null))
        (`GameplayStatics.PlaySound2D` (`self.soundOnActivation`) 1.0 1.0 0.0 null null)))))

(fn `AfterInteraction`)

(fn `Deactivate`
  (if (not (`self.isLocked`))
    (`self.AfterInteraction`)
    (set `self.isActive` false)
    (`self.RenderOutline` false)))

(fn `OnInteraction`)

(fn `RenderOutline`
  (params (value :type Boolean) (bypassLock :type Boolean))
  (if (and (`self.isLocked`) (not bypassLock))
    (bind _asbp_game_state (cast `/Game/Blueprints/BP_GameState` (`GameplayStatics.GetGameState`) :!label _label))
    (`/Game/Blueprints/BP_GameState.ShowHUDInteract` _asbp_game_state "Hidden")
    (else
      (`PrimitiveComponent.SetRenderCustomDepth` (`self.StaticMesh`) value)
      (if value
        (if (`self.showInteractMessage`)
          (bind _asbp_game_state_2 (cast `/Game/Blueprints/BP_GameState` (`GameplayStatics.GetGameState`)))
          (`/Game/Blueprints/BP_GameState.ShowHUDInteract` _asbp_game_state_2 "Visible")
          (else
            (goto _label)))
        (else
          (goto _label))))))

(fn `SetLocked`
  (params (value :type Boolean))
  (set `self.isLocked` value))

(fn `UserConstructionScript`)