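; Pressure plate interactable that switches a set of linked trigger objects on and off.
; On BeginPlay it enables activation on collision and copies its TogglePressurePlate setting into IsToggle.
; OnInteraction calls Activate on every entry in TriggerObjects, and AfterInteraction calls Deactivate on each.
; Collision detection and toggle handling are not in this graph, which only sets those flags and supplies the two interaction responses.
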(event `self.ReceiveBeginPlay`
  (set `self.activationOnCollision` true)
  (set `self.isToggle` (`self.togglePressurePlate`)))

(fn `AfterInteraction`
  (for _array_element (`self.triggerObjects`)
    (`self.Deactivate` _array_element)))

(fn `OnInteraction`
  (for _array_element (`self.triggerObjects`)
    (`self.Activate` _array_element)))

(fn `UserConstructionScript`
  (`parent.UserConstructionScript`))