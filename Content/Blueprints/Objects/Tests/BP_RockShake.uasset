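; Rock obstacle that plays a one-time cutscene of two rocks shaking and sinking into the ground before they are destroyed.
; Tick polls IsActive through a DoOnce, then blends the camera to this actor and disables player input.
; After a delay, timelines drive the roll shake, then a cumulative swept Z offset.
; One second later, the view blends back to the player, input returns and both rock components are destroyed.
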(event `self.ReceiveTick`
  (params (DeltaSeconds :type "Float (single-precision)"))
  (if (`self.isActive`)
    (`/Engine/EditorBlueprintResources/StandardMacros.DoOnce` false
      (:`Completed`
        (`self.CameraPanToRocks`)
        (`KismetSystemLibrary.Delay` (`self.delayUntilShake`))
        (bind (_direction _rock_roll) (`Timeline|ShakeRock`)
          (:`Update`
            (`self.RockMeshShakeOnXAxis` _rock_roll _rock_roll))
          (:`Finished`
            (bind (_direction_2 _rock_disappearing_into_ground) (`Timeline|Rock Drop`)
              (:`Update`
                (`self.RockMeshToNegativeZ` _rock_disappearing_into_ground _rock_disappearing_into_ground))
              (:`Finished`
                (`KismetSystemLibrary.Delay` 1.0)
                (`self.CameraPanToCharacter`)
                (`ActorComponent.K2_DestroyComponent` (`self.Rock1`))
                (`ActorComponent.K2_DestroyComponent` (`self.Rock2`))))))))))

(fn `CameraPanToCharacter`
  (`PlayerController.SetViewTargetWithBlend` (`GameplayStatics.GetPlayerController` 0) (`GameplayStatics.GetPlayerPawn` 0) (`self.blendToPlayer`) "VTBlend_Linear" 0.0 false)
  (`self.EnableInput` (`GameplayStatics.GetPlayerCharacter` 0) (`GameplayStatics.GetPlayerController` 0)))

(fn `CameraPanToRocks`
  (`PlayerController.SetViewTargetWithBlend` (`GameplayStatics.GetPlayerController` 0) self (`self.blendToRocks`) "VTBlend_Linear" 0.0 false)
  (`self.DisableInput` (`GameplayStatics.GetPlayerCharacter` 0) (`GameplayStatics.GetPlayerController` 0)))

(fn `RockMeshShakeOnXAxis`
  (params (NewRotation_Roll :type "Float (double-precision)") (InputPin :type "Float (double-precision)"))
  (bind _rock1 (`self.Rock1`))
  (bind _rock2 (`self.Rock2`))
  (bind (_returnvalue_roll _returnvalue_pitch _returnvalue_yaw) (`KismetMathLibrary.BreakRotator` (`SceneComponent.K2_GetComponentRotation` _rock1)))
  (bind (_returnvalue_roll_2 _returnvalue_pitch_2 _returnvalue_yaw_2) (`KismetMathLibrary.BreakRotator` (`SceneComponent.K2_GetComponentRotation` _rock2)))
  (`SceneComponent.K2_SetWorldRotation` _rock1 (`KismetMathLibrary.MakeRotator` NewRotation_Roll _returnvalue_pitch _returnvalue_yaw) true false)
  (`SceneComponent.K2_SetWorldRotation` _rock2 (`KismetMathLibrary.MakeRotator` InputPin _returnvalue_pitch_2 _returnvalue_yaw_2) true false))

(fn `RockMeshToNegativeZ`
  (params (rock1ToZLocation :type "Float (double-precision)") (rock2ToZLocation :type "Float (double-precision)"))
  (bind _rock1 (`self.Rock1`))
  (bind _rock2 (`self.Rock2`))
  (bind (_returnvalue_x _returnvalue_y _returnvalue_z) (`KismetMathLibrary.BreakVector` (`SceneComponent.K2_GetComponentLocation` _rock2)))
  (bind (_returnvalue_x_2 _returnvalue_y_2 _returnvalue_z_2) (`KismetMathLibrary.BreakVector` (`SceneComponent.K2_GetComponentLocation` _rock1)))
  (`SceneComponent.K2_SetWorldLocation` _rock1 (`KismetMathLibrary.MakeVector` _returnvalue_x_2 _returnvalue_y_2 (+ _returnvalue_z_2 rock1ToZLocation)) true false)
  (`SceneComponent.K2_SetWorldLocation` _rock2 (`KismetMathLibrary.MakeVector` _returnvalue_x _returnvalue_y (+ _returnvalue_z rock2ToZLocation)) true false))

(fn `UserConstructionScript`
  (`parent.UserConstructionScript`))