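; End-game rune that counts toward the game state's collected runes and locks itself when interacted with.
; While active, Tick fades its audio and plays a celebration: player input and bobbing are disabled, IsHappy is set, and the player mesh spins and rises.
; Two timelines, with play rates set in the construction script, drive the motion from start values captured once.
; When the lift finishes, input and bobbing return and IsHappy clears.
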(event `self.ReceiveTick`
  (params (DeltaSeconds :type "Float (single-precision)"))
  (bind _returnvalue (`GameplayStatics.GetPlayerController` 0))
  (if (`self.isActive`)
    (`AudioComponent.AdjustVolume` (`self.Audio`) 0.6 0.0 "Linear")
    (bind _asbp_player_character (cast `/Game/Blueprints/Character/BP_PlayerCharacter` (`GameplayStatics.GetPlayerCharacter` 0)))
    (if (`self.liftFinished`)
      (`/Engine/EditorBlueprintResources/StandardMacros.DoOnce` true :!label _label
        (:`Completed`
          (`/Game/Blueprints/Character/BP_PlayerCharacter.EnableBobbing` _asbp_player_character true)
          (`self.EnableInput` _asbp_player_character _returnvalue)
          (set `/Game/Blueprints/Character/BP_PlayerCharacter.isHappy` false _asbp_player_character)))
      (else
        (`self.Rotate`)
        (`self.Lift`)
        (`/Engine/EditorBlueprintResources/StandardMacros.DoOnce` false
          (:`Completed`
            (`/Game/Blueprints/Character/BP_PlayerCharacter.DisableBobbing` _asbp_player_character true)
            (`self.DisableInput` _asbp_player_character _returnvalue)
            (set `/Game/Blueprints/Character/BP_PlayerCharacter.isHappy` true _asbp_player_character)
            (goto _label :!via `Reset`)))))))

(event `Rotate`
  (`self.SetStartRot`)
  (bind (_direction _spinmultiplier) (`Timeline|Spin Multiplier`)
    (:`Update`
      (bind (_returnvalue_roll _returnvalue_pitch _returnvalue_yaw) (`KismetMathLibrary.BreakRotator` (`SceneComponent.K2_GetComponentRotation` (`Character.Mesh` (stale `self.ReceiveTick` _asbp_player_character)))))
      (`SceneComponent.K2_SetWorldRotation` (`Character.Mesh` (stale `self.ReceiveTick` _asbp_player_character)) (`KismetMathLibrary.MakeRotator` _returnvalue_roll _returnvalue_pitch (+ (* (`self.lapsToSpin`) _spinmultiplier) (`self.startRotation`))) false false))
    (:`Finished`
      (set `self.rotationFinished` true))))

(event `SetStartRot`
  (`/Engine/EditorBlueprintResources/StandardMacros.DoOnce` false
    (:`Completed`
      (bind (_returnvalue_roll _returnvalue_pitch _returnvalue_yaw) (`KismetMathLibrary.BreakRotator` (`SceneComponent.K2_GetComponentRotation` (`Character.Mesh` (stale `self.ReceiveTick` _asbp_player_character)))))
      (set `self.startRotation` _returnvalue_yaw))))

(event `Lift`
  (`self.SetStartPos`)
  (bind (_direction _liftmultiplier) (`Timeline|Lift Multiplier`)
    (:`Update`
      (bind (_returnvalue_x _returnvalue_y _returnvalue_z) (`KismetMathLibrary.BreakVector` (`SceneComponent.K2_GetComponentLocation` (`Character.Mesh` (stale `self.ReceiveTick` _asbp_player_character)))))
      (`SceneComponent.K2_SetWorldLocation` (`Character.Mesh` (stale `self.ReceiveTick` _asbp_player_character)) (`KismetMathLibrary.MakeVector` _returnvalue_x _returnvalue_y (+ (* (`self.liftHeight`) _liftmultiplier) (`self.startPos`))) false false))
    (:`Finished`
      (set `self.liftFinished` true))))

(event `SetStartPos`
  (`/Engine/EditorBlueprintResources/StandardMacros.DoOnce` false
    (:`Completed`
      (bind (_returnvalue_x _returnvalue_y _returnvalue_z) (`KismetMathLibrary.BreakVector` (`SceneComponent.K2_GetComponentLocation` (`Character.Mesh` (stale `self.ReceiveTick` _asbp_player_character)))))
      (set `self.startPos` _returnvalue_z))))

(fn `OnInteraction`
  (bind _asbp_game_state (cast `/Game/Blueprints/BP_GameState` (`GameplayStatics.GetGameState`)))
  (bind _result (`/Engine/EditorBlueprintResources/StandardMacros.IncrementInt` (`/Game/Blueprints/BP_GameState.runesCollected` _asbp_game_state))
    (:`  `
      (set `/Game/Blueprints/BP_GameState.runesCollected` _result _asbp_game_state)
      (`self.SetLocked` true))))

(fn `UserConstructionScript`
  (`parent.UserConstructionScript`)
  (`TimelineComponent.SetPlayRate` (`self.Lift Multiplier`) (`self.liftSpeed`))
  (`TimelineComponent.SetPlayRate` (`self.Spin Multiplier`) (`self.spinSpeed`)))