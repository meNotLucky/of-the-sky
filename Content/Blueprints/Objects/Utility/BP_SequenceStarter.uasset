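; BP_SequenceStarter is a one-shot trigger actor that plays a cutscene on its first overlap, without filtering the overlapping actor.
; It plays the assigned SequenceInitiated sequence and disables player input for a delay set by SequenceTime rather than a finish event.
; It then restores input or, when IsEnd is set, shows the WB_Thanks widget briefly, clears all widgets and opens the SterfanBuild level.
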(event `self.ReceiveActorBeginOverlap`
  (params (OtherActor :type "Actor Object Reference"))
  (`/Engine/EditorBlueprintResources/StandardMacros.DoOnce` false
    (:`Completed`
      (`MovieSceneSequencePlayer.Play` (`LevelSequenceActor.SequencePlayer` (`self.sequenceInitiated`)))
      (`self.DisableInput` (`GameplayStatics.GetPlayerCharacter` 0) (`GameplayStatics.GetPlayerController` 0))
      (`KismetSystemLibrary.Delay` (`self.sequenceTime`))
      (if (`self.isEnd`)
        (bind _returnvalue (`|CreateWidget` "/Game/Blueprints/UI/WB_Thanks.WB_Thanks_C"))
        (`UserWidget.AddToViewport` _returnvalue 10)
        (`KismetSystemLibrary.Delay` 5.0)
        (`WidgetLayoutLibrary.RemoveAllWidgets`)
        (`GameplayStatics.OpenLevel` "SterfanBuild")
        (else
          (`self.EnableInput` (`GameplayStatics.GetPlayerCharacter` 0) (`GameplayStatics.GetPlayerController` 0)))))))

(fn `UserConstructionScript`)