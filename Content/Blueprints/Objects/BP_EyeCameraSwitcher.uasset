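; Interactable eye object that temporarily switches the player's view to itself to show a puzzle and highlight its statues.
; While IsActive, Tick runs a DoOnce-gated sequence that blends to this view, disables character input and makes StatuesToGlow glow.
; After a timed hold it blends back, re-enables input, then clears the glow, restores the interact message and resets the gate.
; OnInteraction only hides the interact message.
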(event `self.ReceiveTick`
  (params (DeltaSeconds :type "Float (single-precision)"))
  (if (`self.isActive`)
    (`/Engine/EditorBlueprintResources/StandardMacros.DoOnce` false :!label _label
      (:`Completed`
        (`PlayerController.SetViewTargetWithBlend` (`GameplayStatics.GetPlayerController` 0) self (`self.blendTimeToCamera`) "VTBlend_Linear" 0.0 false)
        (`self.DisableInput` (`GameplayStatics.GetPlayerCharacter` 0) (`GameplayStatics.GetPlayerController` 0))
        (for _array_element (`self.statuesToGlow`)
          (set `/Game/Blueprints/Puzzles/BP_Statue.glow` true _array_element))
        (`KismetSystemLibrary.Delay` (`self.timeInPuzzleView`))
        (`PlayerController.SetViewTargetWithBlend` (`GameplayStatics.GetPlayerController` 0) (`GameplayStatics.GetPlayerPawn` 0) (`self.blendTimeToPlayer`) "VTBlend_Linear" 0.0 false)
        (`KismetSystemLibrary.Delay` (`self.blendTimeToPlayer`))
        (`self.EnableInput` (`GameplayStatics.GetPlayerCharacter` 0) (`GameplayStatics.GetPlayerController` 0))
        (`KismetSystemLibrary.Delay` (`self.blendTimeToPlayer`))
        (for _array_element_2 (`self.statuesToGlow`)
          (set `/Game/Blueprints/Puzzles/BP_Statue.glow` false _array_element_2)
          (set `self.showInteractMessage` true))
        (goto _label :!via `Reset`)))))

(fn `OnInteraction`
  (set `self.showInteractMessage` false))

(fn `UserConstructionScript`
  (`parent.UserConstructionScript`))