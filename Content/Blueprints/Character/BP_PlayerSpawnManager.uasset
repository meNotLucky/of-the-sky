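; Player respawn manager that returns the player character to a nearby spawn point after it touches the death collider.
; Each tick, while the player is not in the air, it picks the scene component closest to the player mesh as the current spawn, excluding the root and death collider.
; Overlapping the death collider triggers the Death event, which moves the player's root component to that spawn's location.
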(event `self.ReceiveTick`
  (params (DeltaSeconds :type "Float (single-precision)"))
  (bind _returnvalue (`GameplayStatics.GetPlayerCharacter` 0))
  (for _array_element (`self.K2_GetComponentsByClass` "/Script/Engine.SceneComponent")
    (bind _asbp_player_character (cast `/Game/Blueprints/Character/BP_PlayerCharacter` _returnvalue))
    (bind _returnvalue_2 (`KismetMathLibrary.Vector_Distance` (`SceneComponent.K2_GetComponentLocation` _array_element) (`SceneComponent.K2_GetComponentLocation` (`Character.Mesh` _returnvalue))))
    (if (and (not (`/Game/Blueprints/Character/BP_PlayerCharacter.isInAir` _asbp_player_character)) (!= (`self.DefaultSceneRoot`) _array_element) (!= (`self.DeathCollider`) _array_element) (< _returnvalue_2 (`self.previousDistance`)))
      (set `self.previousDistance` _returnvalue_2)
      (set `self.currentSpawn` _array_element)))
  (set `self.previousDistance` 10000000.0))

(event `self.DeathCollider.OnComponentBeginOverlap`
  (params (OverlappedComponent :type "PrimitiveComponent Object Reference") (OtherActor :type "Actor Object Reference") (OtherComp :type "PrimitiveComponent Object Reference") (OtherBodyIndex :type Integer) (bFromSweep :type Boolean) (SweepResult :type "HitResult Structure (by ref)"))
  (if (== OtherActor (`GameplayStatics.GetPlayerCharacter` 0))
    (`self.Death`)))

(event `Death`
  (`SceneComponent.K2_SetWorldLocation` (`Actor.RootComponent` (`GameplayStatics.GetPlayerCharacter` 0)) (`SceneComponent.K2_GetComponentLocation` (`self.currentSpawn`)) false false))

(fn `UserConstructionScript`
  (set `self.previousDistance` 10000000.0))