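; Camera transition actor that opens play with a blend from its own viewpoint to the player character.
; On BeginPlay it snaps player 0's view target to itself, then immediately blends to the character over CameraTransitionSpeed, which serves as the blend duration.
; Character input is disabled during the blend and re-enabled after a Delay of the same length.
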(event `self.ReceiveBeginPlay`
  (`PlayerController.SetViewTargetWithBlend` (`GameplayStatics.GetPlayerController` 0) self 0.0 "VTBlend_Linear" 0.0 false)
  (`self.DisableInput` (`GameplayStatics.GetPlayerCharacter` 0) (`GameplayStatics.GetPlayerController` 0))
  (`PlayerController.SetViewTargetWithBlend` (`GameplayStatics.GetPlayerController` 0) (`GameplayStatics.GetPlayerCharacter` 0) (`self.Camera Transition Speed`) "VTBlend_Linear" 0.0 false)
  (`KismetSystemLibrary.Delay` (`self.Camera Transition Speed`))
  (`self.EnableInput` (`GameplayStatics.GetPlayerCharacter` 0) (`GameplayStatics.GetPlayerController` 0)))

(fn `UserConstructionScript`)