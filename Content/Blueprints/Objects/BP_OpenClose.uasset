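; BP_OpenClose is an interactable bridge that toggles open and closed by rotating its pivot 90 degrees.
; OnInteraction flags an open or close and computes the target rotation, changing roll or yaw according to the direction enum.
; Tick runs the SetBridge macro, which eases the pivot with RInterpTo at a configurable speed.
; Once within one degree of the target, the macro fires End, updating the open state and clearing the flag.
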(event `self.ReceiveTick`
  (params (DeltaSeconds :type "Float (single-precision)"))
  (if (`self.isOpen`)
    (if (`self.closeBridge`)
      (`self.SetBridge`
        (:`End`
          (set `self.isOpen` false)
          (set `self.closeBridge` false))))
    (elif (`self.openBridge`)
      (`self.SetBridge`
        (:`End`
          (set `self.isOpen` true)
          (set `self.openBridge` false))))))

(fn `OnInteraction`
  (bind _returnvalue (== (`self.opencloseDirection`) (enumliteral `/Game/Blueprints/Objects/E_Direction` "NewEnumerator1")))
  (bind (_returnvalue_roll _returnvalue_pitch _returnvalue_yaw) (`KismetMathLibrary.BreakRotator` (`SceneComponent.K2_GetComponentRotation` (`self.BridgePivot`))))
  (bind (_returnvalue_roll_2 _returnvalue_pitch_2 _returnvalue_yaw_2) (`KismetMathLibrary.BreakRotator` (`SceneComponent.K2_GetComponentRotation` (`self.BridgePivot`))))
  (if (`self.isOpen`)
    (if (not (`self.closeBridge`))
      (set `self.closeBridge` true)
      (if _returnvalue
        (set `self.targetRotation` (`KismetMathLibrary.MakeRotator` (+ _returnvalue_roll 90.0) _returnvalue_pitch _returnvalue_yaw))
        (else
          (set `self.targetRotation` (`KismetMathLibrary.MakeRotator` _returnvalue_roll_2 _returnvalue_pitch_2 (+ _returnvalue_yaw_2 90.0))))))
    (elif (not (`self.openBridge`))
      (set `self.openBridge` true)
      (if _returnvalue
        (set `self.targetRotation` (`KismetMathLibrary.MakeRotator` (- _returnvalue_roll 90.0) _returnvalue_pitch _returnvalue_yaw))
        (else
          (set `self.targetRotation` (`KismetMathLibrary.MakeRotator` _returnvalue_roll_2 _returnvalue_pitch_2 (- _returnvalue_yaw_2 90.0))))))))

(fn `UserConstructionScript`
  (`parent.UserConstructionScript`))