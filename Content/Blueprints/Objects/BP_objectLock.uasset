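; BP_objectLock is a socket that captures a designated ObjectToLock and activates linked objects once it is in place.
; Each Tick toggles custom depth rendering on the Lock component to match whether ObjectToLock is active.
; Within 100 units of the Lock, the object is deactivated, marked locked and eased toward it with VInterpTo.
; A DoOnce activates every entry in ObjectsToAcivate when capture begins, without waiting for the snap to finish.
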(event `self.ReceiveTick`
  (params (DeltaSeconds :type "Float (single-precision)"))
  (bind _lock (`self.Lock`))
  (bind _objecttolock (`self.ObjectToLock`))
  (if (`/Game/Blueprints/Objects/Utility/BP_InteractableObject.isActive` (`self.ObjectToLock`))
    (`PrimitiveComponent.SetRenderCustomDepth` _lock true)
    (else
      (`PrimitiveComponent.SetRenderCustomDepth` _lock false)))
  (if (< (`KismetMathLibrary.Vector_Distance` (`SceneComponent.K2_GetComponentLocation` (`/Game/Blueprints/Objects/Utility/BP_InteractableObject.StaticMesh` (`self.ObjectToLock`))) (`SceneComponent.K2_GetComponentLocation` (`self.Lock`))) 100.0)
    (`/Game/Blueprints/Objects/Utility/BP_InteractableObject.Deactivate` _objecttolock)
    (`/Game/Blueprints/Objects/Utility/BP_InteractableObject.SetLocked` _objecttolock true)
    (`SceneComponent.K2_SetWorldLocation` (`/Game/Blueprints/Objects/Utility/BP_InteractableObject.StaticMesh` (`self.ObjectToLock`)) (`KismetMathLibrary.VInterpTo` (`SceneComponent.K2_GetComponentLocation` (`/Game/Blueprints/Objects/Utility/BP_InteractableObject.StaticMesh` (`self.ObjectToLock`))) (`SceneComponent.K2_GetComponentLocation` (`self.Lock`)) (`GameplayStatics.GetWorldDeltaSeconds`) 5.0) false false)
    (`/Engine/EditorBlueprintResources/StandardMacros.DoOnce` false
      (:`Completed`
        (for _array_element (`self.objectsToAcivate`)
          (`/Game/Blueprints/Objects/Utility/BP_InteractableObject.Activate` _array_element))))))

(fn `UserConstructionScript`)