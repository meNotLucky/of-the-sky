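; Long pressure plate interactable that activates its linked trigger objects and glows when triggered by collision, with optional toggle behaviour.
; Interaction activates the trigger objects and raises the glow on a dynamic material created at construction.
; After interaction it plays a sound, deactivates them and clears the glow.
; With LockOnActivation set, it locks on activation, then Tick hides the outline after a delay and disables ticking.
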(event `self.ReceiveBeginPlay`
  (set `self.activationOnCollision` true)
  (set `self.isToggle` (`self.togglePressurePlate`)))

(event `self.ReceiveTick`
  (params (DeltaSeconds :type "Float (single-precision)"))
  (if (`self.lockOnActivation`)
    (if (`self.isActive`)
      (`KismetSystemLibrary.Delay` 2.0)
      (`self.RenderOutline` false true)
      (`self.SetActorTickEnabled` false))))

(fn `AfterInteraction`
  (`GameplayStatics.PlaySound2D` (`self.soundOnDeactivation`) 1.0 1.0 0.0 null null)
  (for _array_element (`self.triggerObjects`)
    (`self.Deactivate` _array_element))
  (`MaterialInstanceDynamic.SetScalarParameterValue` (`self.dynamicMaterial`) "GlowStrenght" 0.0))

(fn `OnInteraction`
  (for _array_element (`self.triggerObjects`)
    (`self.Activate` _array_element))
  (`MaterialInstanceDynamic.SetScalarParameterValue` (`self.dynamicMaterial`) "GlowStrenght" 300.0)
  (if (`self.lockOnActivation`)
    (`self.SetLocked` true)))

(fn `UserConstructionScript`
  (`parent.UserConstructionScript`)
  (bind _returnvalue (`PrimitiveComponent.CreateDynamicMaterialInstance` (`self.StaticMesh`) 0 "/Game/Materials/m_cleanstone_statueglow.m_cleanstone_statueglow" "None"))
  (set `self.dynamicMaterial` _returnvalue))