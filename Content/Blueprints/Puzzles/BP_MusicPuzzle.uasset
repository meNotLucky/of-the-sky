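; BP_MusicPuzzle is a sequence puzzle where the pressure plates in Order must be activated in array order.
; Tick polls the plates, locking correctly activated ones and resetting all with a lose sound if one's predecessor is inactive.
; An active last plate fires Completed once, activating TriggerObjects, switching off long pressure plates, playing a win sound and starting background music after a short delay.
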(event `self.ReceiveTick`
  (params (DeltaSeconds :type "Float (single-precision)"))
  ;[1 1 1] Check Combination
  (for (_array_element _array_index) (`self.order`)
    (if (`/Game/Blueprints/Objects/Utility/BP_InteractableObject.isActive` _array_element)
      (if (== 0 _array_index)
        (if (== (- (`KismetArrayLibrary.Array_Length` (`self.order`)) 1) _array_index) :!label _label
          (`self.Completed`))
        (`/Game/Blueprints/Objects/Utility/BP_InteractableObject.SetLocked` _array_element true)
        (elif (`/Game/Blueprints/Objects/Utility/BP_InteractableObject.isActive` (`|GetArrayItem` (`self.order`) (- _array_index 1)))
          (goto _label)
          (else
            (`self.Reset`)))))))

(event `Reset`
  ;[1 1 1] Reset
  (for _array_element (`self.order`)
    (set `/Game/Blueprints/Objects/Utility/BP_InteractableObject.isActive` false _array_element)
    (`/Game/Blueprints/Objects/Utility/BP_InteractableObject.RenderOutline` _array_element false true)
    (`/Game/Blueprints/Objects/Utility/BP_InteractableObject.SetLocked` _array_element false)
    (`MaterialInstanceDynamic.SetScalarParameterValue` (`/Game/Blueprints/Objects/BP_PressurePlateLong.dynamicMaterial` _array_element) "GlowStrenght" 0.0))
  (`GameplayStatics.PlaySound2D` (`self.puzzleLoseSound`) 1.0 1.0 0.0 null null))

(event `Completed`
  ;[1 1 1] Completed
  (`/Engine/EditorBlueprintResources/StandardMacros.DoOnce` false
    (:`Completed`
      (for _array_element (`self.triggerObjects`)
        (`/Game/Blueprints/Objects/Utility/BP_InteractableObject.Activate` _array_element))
      (for _array_element_2 (`self.order`)
        (bind _asbp_pressure_plate_long (cast `/Game/Blueprints/Objects/BP_PressurePlateLong` _array_element_2))
        (`/Game/Blueprints/Objects/Utility/BP_InteractableObject.SetLocked` _asbp_pressure_plate_long false)
        (`/Game/Blueprints/Objects/Utility/BP_InteractableObject.Deactivate` _asbp_pressure_plate_long)
        (`self.SetActorTickEnabled` _asbp_pressure_plate_long false)
        (`/Game/Blueprints/Objects/Utility/BP_InteractableObject.SetLocked` _asbp_pressure_plate_long false)
        (`self.SetActorTickEnabled` false))
      (`GameplayStatics.PlaySound2D` (`self.puzzleWinSound`) 1.0 1.0 0.0 null null)
      (`KismetSystemLibrary.Delay` 1.0)
      (`/Engine/EditorBlueprintResources/StandardMacros.IsValid` (`self.backgroundMusic`)
        (:`Is Valid`
          (`ActorComponent.Activate` (`AmbientSound.AudioComponent` (`self.backgroundMusic`)) false))))))

(fn `UserConstructionScript`)