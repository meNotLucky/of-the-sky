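; BP_FloatingIsland is an interactable object that raises a referenced island to an end position.
; OnInteraction starts the movement and sets IsLocked.
; While moving, Tick uses VInterpTo at FloatUpSpeed to ease the island's root component toward the EndPositon location, without sweeping, and never clears the MoveUp flag.
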(event `self.ReceiveTick`
  (params (DeltaSeconds :type "Float (single-precision)"))
  (if (`self.moveUp`)
    (`SceneComponent.K2_SetWorldLocation` (`Actor.RootComponent` (`self.island`)) (`KismetMathLibrary.VInterpTo` (`SceneComponent.K2_GetComponentLocation` (`Actor.RootComponent` (`self.island`))) (`SceneComponent.K2_GetComponentLocation` (`self.EndPositon`)) DeltaSeconds (`self.floatUpSpeed`)) false false)))

(fn `OnInteraction`
  (set `self.moveUp` true)
  (set `self.isLocked` true))

(fn `UserConstructionScript`
  (`parent.UserConstructionScript`))