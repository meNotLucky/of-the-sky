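; Large movable object that the player can grab, carry and set down, built on inherited interaction logic.
; Interaction enables physics and switches the player's mode; while grabbed, Tick pushes the mesh with player velocity and eases its height toward the player mesh's Z.
; Release disables physics, traces along the mesh's down vector for a resting height, then eases there, locking interaction and hiding the outline until it settles.
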(event `self.ReceiveTick`
  (params (DeltaSeconds :type "Float (single-precision)"))
  (bind _staticmesh (`self.StaticMesh`))
  (bind _staticmesh_2 (`self.StaticMesh`))
  (bind (_returnvalue_x _returnvalue_y) (`KismetMathLibrary.BreakVector` (`SceneComponent.K2_GetComponentLocation` _staticmesh)))
  (bind (_returnvalue_x_2 _returnvalue_y_2) (`KismetMathLibrary.BreakVector` (`SceneComponent.K2_GetComponentLocation` _staticmesh_2)))
  (set `self.deltaTime` DeltaSeconds)
  (bind _asbp_player_character (cast `/Game/Blueprints/Character/BP_PlayerCharacter` (`GameplayStatics.GetPlayerCharacter` 0)))
  (if (`self.isGrabbed`)
    (bind (_returnvalue_x_3 _returnvalue_y_3 _returnvalue_z) (`KismetMathLibrary.BreakVector` (`SceneComponent.K2_GetComponentLocation` (`Character.Mesh` _asbp_player_character))))
    (set `self.targetObjectZ` _returnvalue_z)
    (`PrimitiveComponent.AddForce` (`self.StaticMesh`) (* (`self.GetVelocity` (`GameplayStatics.GetPlayerCharacter` 0)) 5.5) "None" true)
    (bind _output_get (set `self.currentObjectZ` (`KismetMathLibrary.FInterpTo` (`self.currentObjectZ`) (`self.targetObjectZ`) (`self.deltaTime`) (`self.liftSpeed`))))
    (`SceneComponent.K2_SetWorldLocation` _staticmesh_2 (`KismetMathLibrary.MakeVector` _returnvalue_x_2 _returnvalue_y_2 _output_get) false false)
    (elif (`KismetMathLibrary.NearlyEqual_FloatFloat` (`self.currentObjectZ`) (`self.targetObjectZ`) 0.1)
      (`self.SetLocked` false)
      (else
        (`self.SetLocked` true)
        (bind _output_get_2 (set `self.currentObjectZ` (`KismetMathLibrary.FInterpTo` (`self.currentObjectZ`) (`self.targetObjectZ`) (`self.deltaTime`) (`self.liftSpeed`))))
        (`SceneComponent.K2_SetWorldLocation` _staticmesh (`KismetMathLibrary.MakeVector` _returnvalue_x _returnvalue_y _output_get_2) false false)
        (`self.RenderOutline` false)))))

(fn `AfterInteraction`
  (bind _staticmesh (`self.StaticMesh`))
  (bind _returnvalue (`SceneComponent.K2_GetComponentLocation` _staticmesh))
  (set `self.isGrabbed` false)
  (bind _asbp_player_character (cast `/Game/Blueprints/Character/BP_PlayerCharacter` (`GameplayStatics.GetPlayerCharacter` 0)))
  (set `/Game/Blueprints/Character/BP_PlayerCharacter.mode` "NewEnumerator0" _asbp_player_character)
  (bind _outhit (`KismetSystemLibrary.LineTraceSingle` _returnvalue (+ _returnvalue (* (`SceneComponent.GetUpVector` _staticmesh) -1000.0)) "TraceTypeQuery1"))
  (set `self.targetObjectZ` (+ (- (`self.currentObjectZ`) (`.Distance` (`GameplayStatics.BreakHitResult` _outhit))) (.y (`.BoxExtent` (`KismetSystemLibrary.GetComponentBounds` (`self.StaticMesh`))))))
  (`PrimitiveComponent.SetSimulatePhysics` (`self.StaticMesh`) false))

(fn `OnInteraction`
  (bind (_returnvalue_x _returnvalue_y _returnvalue_z) (`KismetMathLibrary.BreakVector` (`SceneComponent.K2_GetComponentLocation` (`self.StaticMesh`))))
  (set `self.isGrabbed` true)
  (bind _asbp_player_character (cast `/Game/Blueprints/Character/BP_PlayerCharacter` (`GameplayStatics.GetPlayerCharacter` 0)))
  (set `/Game/Blueprints/Character/BP_PlayerCharacter.mode` "NewEnumerator3" _asbp_player_character)
  (`PrimitiveComponent.SetSimulatePhysics` (`self.StaticMesh`) true)
  (bind _output_get (set `self.currentObjectZ` _returnvalue_z))
  (bind _output_get_2 (set `self.startObjectZ` _output_get))
  (set `self.targetObjectZ` _output_get_2))

(fn `UserConstructionScript`
  (`parent.UserConstructionScript`))