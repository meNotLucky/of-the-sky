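; An interactable rune object that counts toward collected runes and starts a cutscene sequence when active.
; Interacting increments RunesCollected on BP_GameState and locks the object.
; Tick watches IsActive and, once, plays the assigned sequence while disabling player input for LookTime.
; Afterward it restores input or, when IsEnd is set, shows a thanks widget and opens the Sterfan4 level.
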(event `self.ReceiveTick`
  (params (DeltaSeconds :type "Float (single-precision)"))
  (if (`self.isActive`)
    (`/Engine/EditorBlueprintResources/StandardMacros.DoOnce` false
      (:`Completed`
        (`MovieSceneSequencePlayer.Play` (`LevelSequenceActor.SequencePlayer` (`self.sequence`)))
        (`self.DisableInput` (`GameplayStatics.GetPlayerCharacter` 0) (`GameplayStatics.GetPlayerController` 0))
        (`KismetSystemLibrary.Delay` (`self.lookTime`))
        (if (`self.isEnd`)
          (bind _returnvalue (`|CreateWidget` "/Game/Blueprints/UI/WB_Thanks.WB_Thanks_C"))
          (`UserWidget.AddToViewport` _returnvalue 0)
          (`KismetSystemLibrary.Delay` 5.0)
          (`WidgetLayoutLibrary.RemoveAllWidgets`)
          (`GameplayStatics.OpenLevel` "Sterfan4")
          (else
            (`self.EnableInput` (`GameplayStatics.GetPlayerCharacter` 0) (`GameplayStatics.GetPlayerController` 0))))))))

(fn `OnInteraction`
  (bind _asbp_game_state (cast `/Game/Blueprints/BP_GameState` (`GameplayStatics.GetGameState`)))
  (bind _result (`/Engine/EditorBlueprintResources/StandardMacros.IncrementInt` (`/Game/Blueprints/BP_GameState.runesCollected` _asbp_game_state))
    (:`  `
      (set `/Game/Blueprints/BP_GameState.runesCollected` _result _asbp_game_state)
      (`self.SetLocked` true))))

(fn `UserConstructionScript`
  (`parent.UserConstructionScript`))