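; Small movable object that the player can pick up, carry and set back down.
; OnInteraction disables mesh collision, and Tick then attaches it to the player while easing its height to just above the player mesh.
; AfterInteraction traces downward for a resting height.
; Tick then detaches it and lowers it while locked with the outline off, unlocking and restoring collision once it settles.
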(event `self.ReceiveTick`
  (params (DeltaSeconds :type "Float (single-precision)"))
  (bind _staticmesh (`self.StaticMesh`))
  (bind _staticmesh_2 (`self.StaticMesh`))
  (bind (_returnvalue_x _returnvalue_y) (`KismetMathLibrary.BreakVector` (`SceneComponent.K2_GetComponentLocation` _staticmesh_2)))
  (bind (_returnvalue_x_2 _returnvalue_y_2) (`KismetMathLibrary.BreakVector` (`SceneComponent.K2_GetComponentLocation` _staticmesh)))
  (set `self.deltaTime` DeltaSeconds)
  (bind _asbp_player_character (cast `/Game/Blueprints/Character/BP_PlayerCharacter` (`GameplayStatics.GetPlayerCharacter` 0)))
  (if (`self.isGrabbed`)
    (bind (_returnvalue_x_3 _returnvalue_y_3 _returnvalue_z) (`KismetMathLibrary.BreakVector` (`SceneComponent.K2_GetComponentLocation` (`Character.Mesh` _asbp_player_character))))
    (set `self.targetObjectZ` (+ _returnvalue_z 50.0))
    (bind _output_get (set `self.currentObjectZ` (`KismetMathLibrary.FInterpTo` (`self.currentObjectZ`) (`self.targetObjectZ`) (`self.deltaTime`) (`self.liftSpeed`))))
    (`SceneComponent.K2_SetWorldLocation` _staticmesh (`KismetMathLibrary.MakeVector` _returnvalue_x_2 _returnvalue_y_2 _output_get) false false)
    (`self.K2_AttachToActor` (`GameplayStatics.GetPlayerCharacter` 0) "None" "KeepWorld" "KeepWorld" "KeepWorld")
    (elif (`KismetMathLibrary.NearlyEqual_FloatFloat` (`self.currentObjectZ`) (`self.targetObjectZ`) 0.1)
      (`self.SetLocked` false)
      (`PrimitiveComponent.SetCollisionEnabled` (`self.StaticMesh`) "QueryAndPhysics")
      (else
        (`self.SetLocked` true)
        (bind _output_get_2 (set `self.currentObjectZ` (`KismetMathLibrary.FInterpTo` (`self.currentObjectZ`) (`self.targetObjectZ`) (`self.deltaTime`) (`self.liftSpeed`))))
        (`SceneComponent.K2_SetWorldLocation` _staticmesh_2 (`KismetMathLibrary.MakeVector` _returnvalue_x _returnvalue_y _output_get_2) false false)
        (`self.K2_DetachFromActor` "KeepWorld" "KeepWorld" "KeepWorld")
        (`self.RenderOutline` false)))))

(fn `AfterInteraction`
  (bind _staticmesh (`self.StaticMesh`))
  (bind _returnvalue (`SceneComponent.K2_GetComponentLocation` _staticmesh))
  (set `self.isGrabbed` false)
  (bind _asbp_player_character (cast `/Game/Blueprints/Character/BP_PlayerCharacter` (`GameplayStatics.GetPlayerCharacter` 0)))
  (set `/Game/Blueprints/Character/BP_PlayerCharacter.mode` "NewEnumerator0" _asbp_player_character)
  (bind _outhit (`KismetSystemLibrary.LineTraceSingle` _returnvalue (+ _returnvalue (* (`SceneComponent.GetUpVector` _staticmesh) -1000.0)) "TraceTypeQuery1"))
  (set `self.targetObjectZ` (+ (- (`self.currentObjectZ`) (`.Distance` (`GameplayStatics.BreakHitResult` _outhit))) 1.0)))

(fn `OnInteraction`
  (bind (_returnvalue_x _returnvalue_y _returnvalue_z) (`KismetMathLibrary.BreakVector` (`SceneComponent.K2_GetComponentLocation` (`self.StaticMesh`))))
  (set `self.isGrabbed` true)
  (bind _asbp_player_character (cast `/Game/Blueprints/Character/BP_PlayerCharacter` (`GameplayStatics.GetPlayerCharacter` 0)))
  (set `/Game/Blueprints/Character/BP_PlayerCharacter.mode` "NewEnumerator0" _asbp_player_character)
  (bind _output_get (set `self.startObjectZ` _returnvalue_z))
  (bind _output_get_2 (set `self.currentObjectZ` _output_get))
  (set `self.targetObjectZ` _output_get_2)
  (`PrimitiveComponent.SetCollisionEnabled` (`self.StaticMesh`) "NoCollision"))

(fn `UserConstructionScript`
  (`parent.UserConstructionScript`))